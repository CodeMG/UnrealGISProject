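; Road generator that builds splines in its construction script from WKT coordinates in the CleanedBigRoadTable data table, over a fixed row index range.
; Parsed points are re-centred, scaled and offset, then line-traced downward and placed slightly above the hit height.
; The trace result is not checked, as the branch is hardwired true.
; When GenerateMesh is set, collidable spline meshes fill each spline in SectionLength steps, with tangents clamped to that length.
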(fn `GetEndAndTangent`
  (params (Spline :type "SplineComponent Object Reference") (Index :type Integer))
  (returns (Position :type "Vector Structure") (Tangent :type "Vector Structure"))
  (bind _returnvalue (* (+ Index 1) (`self.SectionLength`)))
  (return (`SplineComponent.GetLocationAtDistanceAlongSpline` Spline _returnvalue "Local") (`KismetMathLibrary.ClampVectorSize` (`SplineComponent.GetTangentAtDistanceAlongSpline` Spline _returnvalue "Local") 0.0 (`self.SectionLength`))))

(fn `GetStartAndTangent`
  (params (Spline :type "SplineComponent Object Reference") (Index :type Integer))
  (returns (Position :type "Vector Structure") (Tangent :type "Vector Structure"))
  (bind _returnvalue (* Index (`self.SectionLength`)))
  (return (`SplineComponent.GetLocationAtDistanceAlongSpline` Spline _returnvalue "Local") (`KismetMathLibrary.ClampVectorSize` (`SplineComponent.GetTangentAtDistanceAlongSpline` Spline _returnvalue "Local") 0.0 (`self.SectionLength`))))

(fn `UserConstructionScript`
  (locals (CurrentSpline :type "SplineComponent Object Reference") (CurrentPoint :type "Vector Structure"))
  (bind _points (`self.Points`))
  (bind _points_2 (`self.Points`))
  (bind _currentspline (`local.CurrentSpline`))
  ; Get each line in the datatable
  (bind _outrownames (`DataTableFunctionLibrary.GetDataTableRowNames` "/Game/Roads/DataSource/CleanedBigRoadTable.CleanedBigRoadTable"))
  (for _index (range 2001)
    (bind _returnvalue (`|GetDataTableRow` "/Game/Roads/DataSource/CleanedBigRoadTable.CleanedBigRoadTable" (`|GetArrayItem` _outrownames _index))
      (:`then`
        (bind _returnvalue_2 (`AddComponent|NODE_AddSplineComponent-0` :`bManualAttachment` true :`RelativeTransform` (`self.GetTransform`)))
        (set `local.CurrentSpline` _returnvalue_2)
        ; For each point, split it into its components
        (for _array_element (`KismetStringLibrary.ParseIntoArray` (`.WKT_7_AC28547542689DFF21957AA5034E9DE0` (break `/Game/Roads/DataSource/RoadData` _returnvalue)) ",")
          (bind _returnvalue_3 (`KismetStringLibrary.ParseIntoArray` _array_element))
          ; Adjust the point position (Should've exported the data better)
          (bind _output_get (set `local.CurrentPoint` (+ (* (- (`KismetMathLibrary.MakeVector` (`KismetStringLibrary.Conv_StringToDouble` (`|GetArrayItem` _returnvalue_3)) (`KismetStringLibrary.Conv_StringToDouble` (`|GetArrayItem` _returnvalue_3 1)) (`KismetStringLibrary.Conv_StringToDouble` (`|GetArrayItem` _returnvalue_3 2))) (620000.0 5300000.0 0.0)) (`self.Scale`)) (`self.Offset`))))
          ; Raycast to adjust height of the points
          (bind _outhit (`KismetSystemLibrary.LineTraceSingleForObjects` :`Start` (`local.CurrentPoint`) :`End` (+ _output_get (0.0 0.0 -1000.0)) :`ObjectTypes` (`self.RayCastObjectTypes`) :`DrawDebugType` "ForDuration"))
          ; If there was a raycast collision, add the point with the updated z to the array, else the old point
          (if true
            (`KismetArrayLibrary.Array_Add` _points (`KismetMathLibrary.MakeVector` (.x (`local.CurrentPoint`)) (.y (`local.CurrentPoint`)) (+ (.z (`.Location` (`GameplayStatics.BreakHitResult` _outhit))) 10.0)))
            (else
              (`KismetArrayLibrary.Array_Add` _points (`local.CurrentPoint`)))))
        ; Once the points have been created, add them to the spline
        (`SplineComponent.SetSplinePoints` _returnvalue_2 _points_2 "Local" true)
        ; Clear the points array, so that the next line can use it again
        (`KismetArrayLibrary.Array_Clear` _points_2)
        (if (`self.GenerateMesh`)
          (for _index_2 (range (+ (`KismetMathLibrary.FTrunc` (/ (`SplineComponent.GetSplineLength` _returnvalue_2) (`self.SectionLength`))) 1))
            ; Create and add the mesh
            (bind _returnvalue_4 (`AddComponent|NODE_AddSplineMeshComponent-1`))
            (`PrimitiveComponent.SetMaterial` _returnvalue_4 0 "/Game/Roads/RoadMaterial.RoadMaterial")
            (`StaticMeshComponent.SetStaticMesh` _returnvalue_4 (`self.SplineMesh`))
            (`SplineMeshComponent.SetForwardAxis` _returnvalue_4 "X" true)
            (bind (_position _tangent) (`self.GetStartAndTangent` _currentspline _index_2))
            (bind (_position_2 _tangent_2) (`self.GetEndAndTangent` _currentspline _index_2))
            (`SplineMeshComponent.SetStartAndEnd` _returnvalue_4 _position _tangent _position_2 _tangent_2 true)
            (`PrimitiveComponent.SetCollisionEnabled` _returnvalue_4 "QueryAndPhysics")))))))